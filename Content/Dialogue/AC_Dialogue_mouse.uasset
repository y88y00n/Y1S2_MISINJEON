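; Dialogue component for a Mouse NPC that asks for cheese, with Korean lines and player choices.
; Overrides Dialogue, calls the parent, then branches on DialogueTreeIndex into nested AddDialogue nodes that advance by State and chosen OptionIndex.
; Endings set the tree index, remove or clear progress, then close the conversation.
; The second tree's random follow-up line always picks the first option, and its choices lead nowhere.
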(fn `Dialogue`
  (`parent.Dialogue`)
  ;[1 1 1] 선택지
  (switch `int` (`self.DialogueTreeIndex`)
    (:`0`
      ;[1 1 1] 선택지1
      (bind (_state _optionindex) (`self.AddDialogue` "Mouse" "안녕 치즈 좀 주라 쥑쥑" (`|MakeArray` "응줄게" "응싫어" :!type "Text")))
      (switch `/Game/Dialogue/Enum_Dialogue` _state
        (:`NewEnumerator0`
          (switch `int` _optionindex
            (:`0`
              (bind (_state_2 _optionindex_2) (`self.AddDialogue` "Mouse" "감사합니다" (`|MakeArray` "치즈를 준다" "주지 않는다" :!type "Text")))
              (switch `/Game/Dialogue/Enum_Dialogue` _state_2
                (:`NewEnumerator0`
                  (switch `int` _optionindex_2
                    (:`0`
                      (bind _state_3 (`self.AddDialogue` "Mouse" "은혜를 갚을게요" (`|MakeArray` "계속" :!type "Text")))
                      (switch `/Game/Dialogue/Enum_Dialogue` _state_3
                        (:`NewEnumerator0`
                          (`self.SetDialogueTreeIndex` 0)
                          (`self.CloseConversation`))))
                    (:`1`
                      (bind _state_4 (`self.AddDialogue` "Mouse" "진심 감사" (`|MakeArray` "계속" :!type "Text")))
                      (switch `/Game/Dialogue/Enum_Dialogue` _state_4
                        (:`NewEnumerator0`
                          ;[1 1 1] 대화가 끝나고 돌아갈 곳
                          (`self.RemoveDialogueProgress` 2)
                          (`self.CloseConversation`))))))))
            (:`1`
              (bind _state_5 (`self.AddDialogue` "Mouse" "이 일을 후회하게 될 것이다" (`|MakeArray` "계속" :!type "Text")))
              (switch `/Game/Dialogue/Enum_Dialogue` _state_5
                (:`NewEnumerator0`
                  (`self.ClearDialogueProgress`)
                  (`self.CloseConversation`))))))))
    (:`1`
      ;[1 1 1] 선택지2
      (bind _state_6 (`self.AddDialogue` "Mouse" (select `int` (`KismetMathLibrary.RandomIntegerInRange` 0) :`0` "방금 치즈 고마웠어!" :`1` "근데 혹시 더 있어?" :!type "Text") (`|MakeArray` "응줄게" "응싫어" :!type "Text")))
      (switch `/Game/Dialogue/Enum_Dialogue` _state_6))))